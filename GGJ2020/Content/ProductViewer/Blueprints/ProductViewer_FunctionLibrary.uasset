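; Function library for the Product Viewer with helpers for actor tags, actor hierarchies and menu buttons.
; FindTagInfo finds a "Transform" tag and parses its "+"-delimited location, rotation and scale into a transform.
; GetAttachedActors walks attachments level by level without recursion, returning parallel actor and parent arrays, with the root as its own parent.
; MakeCustomMenuButton creates a labeled button, binds its click event and adds it to a given menu.
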(fn `FindTagInfo`
  (params (Array :type "Array of Name"))
  (returns (ExistingTagFound :type Boolean) (Index :type Integer) (ExistingTagTransform :type "Transform Structure"))
  (locals (TagFound :type Boolean) (TagIndex :type Integer) (FoundTransorm :type "Transform Structure"))
  (set `local.TagFound` false)
  (for (_array_element _array_index) Array
    (bind _returnvalue (`KismetStringLibrary.Conv_NameToString` _array_element))
    (bind _returnvalue_2 (`KismetStringLibrary.EqualEqual_StrStr` (`KismetStringLibrary.GetSubstring` _returnvalue (`KismetStringLibrary.FindSubstring` _returnvalue "Transform" true) 9) "Transform"))
    (if _returnvalue_2
      (`|ExecutionSequence`
        (:`then_0`
          (break))
        (:`then_1`
          (set `local.TagFound` _returnvalue_2)
          (set `local.TagIndex` _array_index)
          (bind _returnvalue_3 (`KismetStringLibrary.ParseIntoArray` (`KismetStringLibrary.Conv_NameToString` _array_element) "+"))
          (set `local.FoundTransorm` (`KismetMathLibrary.MakeTransform` (`KismetStringLibrary.Conv_StringToVector` (`|GetArrayItem` _returnvalue_3 1)) (`KismetStringLibrary.Conv_StringToRotator` (`|GetArrayItem` _returnvalue_3 2)) (`KismetStringLibrary.Conv_StringToVector` (`|GetArrayItem` _returnvalue_3 3))))))))
  (return (`local.TagFound`) (`local.TagIndex`) (`local.FoundTransorm`)))

(fn `GetAttachedActors`
  (params (InputPin :type "Actor Object Reference (by ref)"))
  (returns (Actor :type "Array of Actor Object Reference") (ParrentActor :type "Array of Actor Object Reference"))
  (locals (ActorArray :type "Array of Actor Object Reference") (NewParentActorsFound :type "Array of Actor Object Reference") (CurrentParentActors :type "Array of Actor Object Reference") (CurrentAttachedActors :type "Array of Actor Object Reference") (ActorParrentArray :type "Array of Actor Object Reference"))
  (`KismetArrayLibrary.Array_Add` (`local.ActorParrentArray`) InputPin)
  (`KismetArrayLibrary.Array_Add` (`local.ActorArray`) InputPin)
  (`KismetArrayLibrary.Array_Add` (`local.NewParentActorsFound`) InputPin)
  (set `local.CurrentParentActors` (`local.NewParentActorsFound`) :!label _label)
  (`KismetArrayLibrary.Array_Clear` (`local.NewParentActorsFound`))
  (if (>= (`KismetArrayLibrary.Array_Length` (`local.CurrentParentActors`)) 1)
    (for _array_element (`local.CurrentParentActors`)
      (bind _output_get (set `local.CurrentAttachedActors` (`Actor.GetAttachedActors` _array_element)))
      (for _array_element_2 _output_get
        (if (>= (`KismetArrayLibrary.Array_Length` (`Actor.GetAttachedActors` _array_element_2)) 1)
          (`KismetArrayLibrary.Array_Add` (`local.NewParentActorsFound`) _array_element_2))
        (`KismetArrayLibrary.Array_Add` (`local.ActorArray`) _array_element_2)
        (`KismetArrayLibrary.Array_Add` (`local.ActorParrentArray`) _array_element)))
    (goto _label)
    (else
      (return (`local.ActorArray`) (`local.ActorParrentArray`)))))

(fn `MakeCustomMenuButton`
  (params (BindEventToClickedButton :type "Delegate (by ref)") (ButtonText :type Text) (CustomMenu :type "/Game/ProductViewer/Blueprints/Widgets/CustomMenu Object Reference"))
  (returns (CurrentButton :type "/Game/ProductViewer/Blueprints/Widgets/MenuButton Object Reference"))
  (bind _returnvalue (`|CreateWidget` "/Game/ProductViewer/Blueprints/Widgets/MenuButton.MenuButton_C"))
  (add `/Game/ProductViewer/Blueprints/Widgets/MenuButton.ClickedButton` _returnvalue BindEventToClickedButton)
  (add `/Game/ProductViewer/Blueprints/Widgets/MenuButton.DoIt` _returnvalue BindEventToClickedButton)
  (`TextBlock.SetText` (`/Game/ProductViewer/Blueprints/Widgets/MenuButton.Button_Text` _returnvalue) ButtonText)
  (`/Game/ProductViewer/Blueprints/Widgets/CustomMenu.AddButton` CustomMenu _returnvalue)
  (return _returnvalue))