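; Product Viewer actor that toggles its static mesh parts between assembled and exploded views.
; Separate events record each part's initial and exploded relative transforms into two arrays, and a timeline lerps between them forward or in reverse.
; Once the Collector reports the pawn created, it adds an Explode/Rebuild button to the pawn's custom menu.
; The button appears on Space while hovered, or when selected with the VR right-hand menu on.
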(event `self.ReceiveBeginPlay`
  ;[1 1 1] BeginPlay
  (`|ExecutionSequence`
    (:`then_0`
      (`self.EnableInput` (`GameplayStatics.GetPlayerController` 0)))
    (:`then_1`
      (`self.Create_Explode_Button`))
    (:`then_2`
      (add `self.OnBeginCursorOver` (delegate `Bind_OnBeginCursorOver`))
      (add `self.OnEndCursorOver` (delegate `CustomEvent`)))
    (:`then_3`
      (`self.View_Initial_Transform`))))

(event `Bind_OnBeginCursorOver` :!signature `self.OnBeginCursorOver`
  (params (TouchedActor :type "Actor Object Reference"))
  ;[1 1 1] BeginPlay
  (set `self.CursorOver` true))

(event `CustomEvent` :!signature `self.OnEndCursorOver`
  (params (TouchedActor :type "Actor Object Reference"))
  ;[1 1 1] BeginPlay
  (set `self.CursorOver` false))

(event `View_Initial_Transform`
  ;[1 1 1] View Initial Transform
  (for (_array_element _array_index) (`self.SelfStaticMeshComponents`)
    (`SceneComponent.K2_SetRelativeTransform` _array_element (`|GetArrayItem` (`self.FirstTransform`) _array_index) false false)))

(event `Set_Explode_Transform`
  ;[1 1 1] Set Explode Parts Transforms
  (`KismetArrayLibrary.Array_Clear` (`self.SecondTransform`))
  (for _array_element (`self.SelfStaticMeshComponents`)
    (`KismetArrayLibrary.Array_Add` (`self.SecondTransform`) (`SceneComponent.GetRelativeTransform` _array_element)))
  (`self.vIEW_Initial_Transform`))

(event `View_Explode_Transform`
  ;[1 1 1] See_Explode_Part
  (if (not (<= (`KismetArrayLibrary.Array_Length` (`self.SecondTransform`)) 0))
    (for (_array_element _array_index) (`self.SelfStaticMeshComponents`)
      (`SceneComponent.K2_SetRelativeTransform` _array_element (`|GetArrayItem` (`self.SecondTransform`) _array_index) false false))))

(event `Explode_Anim`
  (bind _button_text (`/Game/ProductViewer/Blueprints/Widgets/MenuButton.Button_Text` (`self.ExplodeButton`)))
  ;[1 1 1] Explode_Animation
  (if (`self.IsExplode`)
    (bind (_direction _newtrack_0) (`Timeline|Timeline_0` :!via `Reverse` :!label _label)
      (:`Update`
        (for (_array_element _array_index) (`self.SelfStaticMeshComponents`)
          (`SceneComponent.K2_SetRelativeTransform` _array_element (`KismetMathLibrary.TLerp` (`|GetArrayItem` (`self.FirstTransform`) _array_index) (`|GetArrayItem` (`self.SecondTransform`) _array_index) _newtrack_0) false false)))
      (:`Finished`
        (`/Engine/EditorBlueprintResources/StandardMacros.FlipFlop`
          (:`A`
            (set `self.IsExplode` true)
            (`TextBlock.SetText` _button_text "Rebuild"))
          (:`B`
            (set `self.IsExplode` false)
            (`TextBlock.SetText` _button_text "Explode")))))
    (else
      (goto _label))))

(event `self.ReceiveTick`
  (params (DeltaSeconds :type "Float (single-precision)"))
  (bind _explodebutton (`self.ExplodeButton`))
  ;[1 0.3646 0.3646] Tick
  (bind _asproduct_viewer_vr_pawn (cast `/Game/ProductViewer/Blueprints/ProductViewer_VR_Pawn` (`self.ProductViewerBasePawn`)))
  (if (and (`/Game/ProductViewer/Blueprints/ProductViewer_VR_Pawn.RightHandMenuOn` _asproduct_viewer_vr_pawn) (== (`/Game/ProductViewer/Blueprints/ProductViewer_Base_Pawn.CurrentSelectable` _asproduct_viewer_vr_pawn) self))
    (`Widget.SetVisibility` _explodebutton "Visible")
    (`KismetSystemLibrary.RetriggerableDelay` 2.0)
    (`Widget.SetVisibility` _explodebutton "Collapsed")))

(event `Key|SpaceBar` :consume false
  (params (Key :type "Key Structure"))
  ;[1 1 1] Enable Explode Widget
  (:`Pressed`
    (if (`self.CursorOver`)
      (`Widget.SetVisibility` (`self.ExplodeButton`) "Visible")))
  (:`Released`
    (`Widget.SetVisibility` (`self.ExplodeButton`) "Collapsed")
    (set `self.CursorOver` false)))

(event `Set_Initial_Transform`
  ;[1 1 1] Set Initial Transform
  (`KismetArrayLibrary.Array_Clear` (`self.FirstTransform`))
  (for _array_element (`self.SelfStaticMeshComponents`)
    (`KismetArrayLibrary.Array_Add` (`self.FirstTransform`) (`SceneComponent.GetRelativeTransform` _array_element))))

(event `Create_Explode_Button`
  ;[1 1 1] Add Custom Menu Button
  (bind _outactors (`GameplayStatics.GetAllActorsOfClass` "/Game/ProductViewer/Blueprints/ProductViewer_Collector.ProductViewer_Collector_C"))
  (add `/Game/ProductViewer/Blueprints/ProductViewer_Collector.CreatePawnDone` (`|GetArrayItem` _outactors) (delegate `YOYOYO`)))

(event `CustomEvent_0`
  ;[1 1 1] Add Custom Menu Button
  (`self.Explode_Anim`))

(event `YOYOYO`
  ;[1 1 1] Add Custom Menu Button
  (bind _outactors (`GameplayStatics.GetAllActorsOfClass` "/Game/ProductViewer/Blueprints/ProductViewer_Base_Pawn.ProductViewer_Base_Pawn_C"))
  (bind _output (`|GetArrayItem` _outactors))
  (set `self.ProductViewerBasePawn` _output)
  (bind _currentbutton (`/Game/ProductViewer/Blueprints/ProductViewer_FunctionLibrary.MakeCustomMenuButton` (delegate `CustomEvent_0`) "Explode" (`/Game/ProductViewer/Blueprints/ProductViewer_Base_Pawn.CustomMenu` _output)))
  (bind _output_get (set `self.ExplodeButton` _currentbutton))
  (`Widget.SetVisibility` _output_get "Collapsed"))

(event `GetComponents`
  (set `self.SelfStaticMeshComponents` (`self.K2_GetComponentsByClass` "/Script/Engine.StaticMeshComponent")))

(fn `UserConstructionScript`)